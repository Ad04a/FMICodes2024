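; BP_Building is a clickable overworld building that leads into the ComersialUse level.
; On left mouse release it calls DrawLine, then checks IsConnecting on OverWorldGameModeBase.
; If no connection is in progress, it prints its router, decoder and switch counts, then opens the level after a short delay.
; The three counts travel as the level's options string, concatenated without separators.
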(event `self.ReceiveBeginPlay`)

(event `self.ReceiveActorOnReleased`
  (params (ButtonReleased :type "Key Structure"))
  (bind _returnvalue (`KismetStringLibrary.Concat_StrStr` (`KismetStringLibrary.BuildString_Int` "" "" (`self.RouterCount`)) (`KismetStringLibrary.BuildString_Int` "" "" (`self.DecoderCount`)) (`KismetStringLibrary.BuildString_Int` "" "" (`self.SwitchCount`))))
  (if (== ButtonReleased "LeftMouseButton")
    (`self.DrawLine`)
    (bind _asover_world_game_mode_base (cast `OverWorldGameModeBase` (`GameplayStatics.GetGameMode`)))
    (if (not (`KismetMathLibrary.Conv_IntToBool` (`OverWorldGameModeBase.IsConnecting` _asover_world_game_mode_base)))
      (`KismetSystemLibrary.PrintString` _returnvalue true true (struct :`G` 0.66 :`B` 1.0 :`A` 1.0) 2000.0)
      (`KismetSystemLibrary.Delay` 1.5)
      (`GameplayStatics.OpenLevel` "ComersialUse" true _returnvalue))))

(fn `UserConstructionScript`)