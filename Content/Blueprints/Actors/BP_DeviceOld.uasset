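; BP_DeviceOld is a device actor with four HDMI port components that act as connection points for cables, with debug prints throughout.
; Releasing a click on any port prints its name, and hovering over the first port prints a default message.
; Only Hdmi1 handles overlaps: it attaches any overlapping actor to itself with relative transforms, prints that actor's name, then clears IsHeld if it is a BP_CableOld.
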(event `self.hdmi.OnReleased`
  (params (TouchedComponent :type "PrimitiveComponent Object Reference") (ButtonReleased :type "Key Structure"))
  (`KismetSystemLibrary.PrintString` "hdmi" true true (struct :`G` 0.66 :`B` 1.0 :`A` 1.0) 10000.0))

(event `self.hdmi1.OnReleased`
  (params (TouchedComponent :type "PrimitiveComponent Object Reference") (ButtonReleased :type "Key Structure"))
  (`KismetSystemLibrary.PrintString` "hdmi1" true true (struct :`G` 0.66 :`B` 1.0 :`A` 1.0) 10000.0))

(event `self.hdmi2.OnReleased`
  (params (TouchedComponent :type "PrimitiveComponent Object Reference") (ButtonReleased :type "Key Structure"))
  (`KismetSystemLibrary.PrintString` "hdmi2" true true (struct :`G` 0.66 :`B` 1.0 :`A` 1.0) 10000.0))

(event `self.hdmi3.OnReleased`
  (params (TouchedComponent :type "PrimitiveComponent Object Reference") (ButtonReleased :type "Key Structure"))
  (`KismetSystemLibrary.PrintString` "hdmi3" true true (struct :`G` 0.66 :`B` 1.0 :`A` 1.0) 10000.0))

(event `self.hdmi.OnBeginCursorOver`
  (params (TouchedComponent :type "PrimitiveComponent Object Reference"))
  (`KismetSystemLibrary.PrintString` "Hello" true true (struct :`G` 0.66 :`B` 1.0 :`A` 1.0) 100002.0))

(event `self.hdmi1.OnComponentBeginOverlap`
  (params (OverlappedComponent :type "PrimitiveComponent Object Reference") (OtherActor :type "Actor Object Reference") (OtherComp :type "PrimitiveComponent Object Reference") (OtherBodyIndex :type Integer) (bFromSweep :type Boolean) (SweepResult :type "HitResult Structure (by ref)"))
  (`self.K2_AttachToComponent` OtherActor OverlappedComponent "None" "KeepRelative" "KeepRelative" "KeepRelative" true)
  (`KismetSystemLibrary.PrintString` (`KismetSystemLibrary.GetDisplayName` OtherActor) true true (struct :`G` 0.66 :`B` 1.0 :`A` 1.0) 20000.0)
  (bind _asbp_cable_old (cast `/Game/Blueprints/Actors/BP_CableOld` OtherActor))
  (set `/Game/Blueprints/Actors/BP_CableOld.IsHeld` false _asbp_cable_old))

(fn `UserConstructionScript`)