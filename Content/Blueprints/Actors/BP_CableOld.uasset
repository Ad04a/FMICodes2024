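; BP_CableOld is a cable actor meant to be picked up by clicking and moved while held.
; Clicking sets a held flag and stores the player controller's screen mouse position as an X/Z vector with zero Y; releasing clears the flag.
; While held, Tick adds that vector to the actor location, then rebuilds it from their sum, so movement compounds without re-reading the mouse.
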(event `self.ReceiveBeginPlay`
  (set `self.PlayerController` (`GameplayStatics.GetPlayerController` 0)))

(event `self.ReceiveTick`
  (params (DeltaSeconds :type "Float (single-precision)"))
  (bind (_returnvalue_x _returnvalue_y _returnvalue_z) (`KismetMathLibrary.BreakVector` (+ (`self.mousevector`) (`self.K2_GetActorLocation`))))
  (if (`self.IsHeld`)
    (`self.K2_SetActorLocation` (`KismetMathLibrary.MakeVector` _returnvalue_x _returnvalue_y _returnvalue_z))
    (set `self.mousevector` (`KismetMathLibrary.MakeVector` _returnvalue_x 0.0 _returnvalue_z))))

(event `self.ReceiveActorOnClicked`
  (params (ButtonPressed :type "Key Structure"))
  (bind (_locationx _locationy) (`PlayerController.GetMousePosition` (`self.PlayerController`)))
  (set `self.IsHeld` true)
  (set `self.mousevector` (`KismetMathLibrary.MakeVector` _locationx 0.0 _locationy)))

(event `self.ReceiveActorOnReleased`
  (params (ButtonReleased :type "Key Structure"))
  (set `self.IsHeld` false))

(fn `UserConstructionScript`)